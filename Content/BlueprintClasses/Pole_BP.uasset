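; Pole actor for a ring-stacking puzzle, with five slot positions and a RingController that tracks its rings.
; On BeginPlay the starting pole places its rings in those slots and registers them with the controller.
; An overlapping ring highlights the pole through custom depth, and Tick binds to the first-person character's drop event during overlap.
; On drop, the ring goes to the RingController for assessment; RemoveRingActor updates the controller's list, count and pointer.
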(event Custom|OnDrop_Event
  (Utilities|IsValid (Variables|--PrivateAttributes--|GetringActor)
    (:Is%20Valid
      (Default|AssesRingActor (Variables|Default|GetRingController) (Variables|--PrivateAttributes--|GetringActor))
      (Rendering|SetRenderCustomDepth (Variables|Default|GetPoleMesh) false))))

(event EventBeginPlay
  (CallFunction|CompilePositions)
  (CallFunction|ArrangeRings)
  (Variables|/Game/BlueprintClasses/RingController.RingController_C|SetPoleRef (Variables|Default|GetRingController) self)
  (bind _asfirst_person_character (Utilities|Casting|CastToFirstPersonCharacter (Game|GetPlayerCharacter 0)))
  (Variables|--PrivateAttributes--|SetCharRef _asfirst_person_character))

(event Collision|EventActorBeginOverlap
  (params (OtherActor :type Actor%20Object%20Reference))
  (if (CallFunction|IsRingActor OtherActor)
    (bind _asring_actor_inst (Utilities|Casting|CastToRingActor_Inst OtherActor))
    (Variables|--PrivateAttributes--|SetringActor _asring_actor_inst)
    (Rendering|SetRenderCustomDepth (Variables|Default|GetPoleMesh) true)
    (Variables|--PrivateAttributes--|SethasRingActorOverlapped true)))

(event EventTick
  (params (DeltaSeconds :type Float%20%28single-precision%29))
  (if (Variables|--PrivateAttributes--|GethasRingActorOverlapped)
    (EventDispatchers|BindEventtoDropEvent (Variables|--PrivateAttributes--|GetCharRef) (delegate Custom|OnDrop_Event))))

(event Collision|EventActorEndOverlap
  (params (OtherActor :type Actor%20Object%20Reference))
  (if (CallFunction|IsRingActor OtherActor)
    (Rendering|SetRenderCustomDepth (Variables|Default|GetPoleMesh) false)
    (Variables|--PrivateAttributes--|SethasRingActorOverlapped false)
    (Variables|--PrivateAttributes--|SetringActor 0)))

(fn ConstructionScript)

(fn IsRingActor
  (params (Other :type Actor%20Object%20Reference))
  (Utilities|Casting|CastToRingActor_Inst Other
    (:then
      (return true))
    (:CastFailed
      (return false))))

(fn ArrangeRings
  (if (Variables|--EditableAttributes--|GetIsStartingPole)
    (for (_array_element _array_index) (Variables|--PrivateAttributes--|GetRings)
      (Transformation|SetActorLocation _array_element (Transformation|GetWorldLocation (Utilities|Array|Get(acopy) (Variables|--PrivateAttributes--|GetPolePositions) _array_index)) false false))
    (CallFunction|InitializeRingData)))

(fn CompilePositions
  (bind _polepositions (Variables|--PrivateAttributes--|GetPolePositions))
  (Utilities|Array|Add _polepositions (Variables|Default|GetPosition_01))
  (Utilities|Array|Add _polepositions (Variables|Default|GetPosition_02))
  (Utilities|Array|Add _polepositions (Variables|Default|GetPosition_03))
  (Utilities|Array|Add _polepositions (Variables|Default|GetPosition_04))
  (Utilities|Array|Add _polepositions (Variables|Default|GetPosition_05)))

(fn InitializeRingData
  (bind _ringcontroller (Variables|Default|GetRingController))
  (for (_array_element _array_index) (Variables|--PrivateAttributes--|GetRings)
    (Variables|/Game/BlueprintClasses/RingActors/RingActor_Inst.RingActor_Inst_C|SetPoleReference _array_element self)
    (Utilities|Array|Add (Variables|/Game/BlueprintClasses/RingController.RingController_C|GetCurrentRings (Variables|Default|GetRingController)) _array_element)
    (Variables|/Script/TowerOfHanoi_V3.RingActor|SetLastLocation _array_element (Transformation|GetWorldLocation (Variables|/Game/BlueprintClasses/RingActors/RingActor_Inst.RingActor_Inst_C|GetDefaultSceneRoot _array_element)))
    (Variables|/Script/TowerOfHanoi_V3.RingActor|SetPoleIndexID _array_element _array_index))
  (Default|UpdatePointer _ringcontroller)
  (Variables|/Game/BlueprintClasses/RingController.RingController_C|SetcurRingCounter _ringcontroller (Utilities|Array|Length (Variables|/Game/BlueprintClasses/RingController.RingController_C|GetCurrentRings _ringcontroller))))

(fn RemoveRingActor
  (params (RingActor :type Ring%20Actor%20Inst%20Object%20Reference))
  (bind _ringcontroller (Variables|Default|GetRingController))
  (bind _result (Math|Integer|DecrementInt (Variables|/Game/BlueprintClasses/RingController.RingController_C|GetcurRingCounter _ringcontroller))
    (:%20%20
      (Variables|/Game/BlueprintClasses/RingController.RingController_C|SetcurRingCounter _ringcontroller (Math|Integer|Clamp(Integer) _result 0 5))
      (Utilities|Array|RemoveItem (Variables|/Game/BlueprintClasses/RingController.RingController_C|GetCurrentRings (Variables|Default|GetRingController)) RingActor)
      (Default|UpdatePointer (Variables|Default|GetRingController)))))