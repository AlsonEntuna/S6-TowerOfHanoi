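; Table actor that lets the first-person player enter and leave a game mode at the table.
; Overlapping it shows a PlayGame_UMG prompt widget and sets a flag that makes Tick repeatedly bind the character's interact and escape events, with no unbind.
; Interact removes the widget, blends to the table's target view, locks movement and shows the cursor.
; Escape restores the player camera, movement and game-only input.
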(event Custom|OnInteract_Event
  (CallFunction|InitGameModules))

(event Custom|OnEscape_Event
  (CallFunction|FinishGameModules))

(event EventBeginPlay
  (bind _asfirst_person_character (Utilities|Casting|CastToFirstPersonCharacter (Game|GetPlayerCharacter 0)))
  (Variables|--PrivateAttributes--|SetPRef _asfirst_person_character))

(event Collision|EventActorBeginOverlap
  (params (OtherActor :type Actor%20Object%20Reference))
  (if (CallFunction|IsCharacter OtherActor)
    (Variables|--PrivateAttributes--|SetCollided true)
    (bind _returnvalue (UserInterface|CreateWidget "/Game/UMG/PlayGame_UMG.PlayGame_UMG_C"))
    (bind _output_get (Variables|--PrivateAttributes--|SetUIRef _returnvalue))
    (UserInterface|Viewport|AddtoViewport _output_get 0)))

(event Collision|EventActorEndOverlap
  (params (OtherActor :type Actor%20Object%20Reference))
  (bind _uiref (Variables|--PrivateAttributes--|GetUIRef))
  (if (CallFunction|IsCharacter OtherActor)
    (Variables|--PrivateAttributes--|SetCollided false)
    (Utilities|IsValid _uiref
      (:Is%20Valid
        (Widget|RemovefromParent _uiref)))))

(event EventTick
  (params (DeltaSeconds :type Float%20%28single-precision%29))
  (if (Variables|--PrivateAttributes--|GetCollided)
    (EventDispatchers|BindEventtoInteractEvent (Variables|--PrivateAttributes--|GetPRef) (delegate Custom|OnInteract_Event))
    (EventDispatchers|BindEventtoEscapeEvent (Variables|--PrivateAttributes--|GetPRef) (delegate Custom|OnEscape_Event))))

(fn ConstructionScript)

(fn IsCharacter
  (params (Other :type Actor%20Object%20Reference))
  (Utilities|Casting|CastToFirstPersonCharacter Other
    (:then
      (return true))
    (:CastFailed
      (return false))))

(fn InitGameModules
  (bind _returnvalue (Game|GetPlayerController 0))
  (bind _uiref (Variables|--PrivateAttributes--|GetUIRef))
  (Utilities|IsValid _uiref
    (:Is%20Valid
      (Widget|RemovefromParent _uiref)
      (Game|Player|SetViewTargetwithBlend (Game|GetPlayerController 0) (Components|GetOwner (Variables|Default|GetTargetView)) 0.5 "VTBlend_Linear" 0.0 false)
      (Variables|/Script/TowerOfHanoi_V3.TowerOfHanoi_V3Character|SetCanMove (Variables|--PrivateAttributes--|GetPRef) false)
      (Variables|/Script/Engine.PlayerController|SetbShowMouseCursor _returnvalue true)
      (Input|SetInputModeGameandUI _returnvalue 0 false false)
      (Variables|/Game/FirstPersonCPP/Blueprints/FirstPersonCharacter.FirstPersonCharacter_C|SetInGame (Variables|--PrivateAttributes--|GetPRef) true))))

(fn FinishGameModules
  (bind _returnvalue (Game|GetPlayerController 0))
  (Game|Player|SetViewTargetwithBlend (Game|GetPlayerController 0) (Components|GetOwner (Variables|/Game/FirstPersonCPP/Blueprints/FirstPersonCharacter.FirstPersonCharacter_C|GetMainCamera (Variables|--PrivateAttributes--|GetPRef))) 0.5 "VTBlend_Linear" 0.0 false)
  (Variables|/Script/TowerOfHanoi_V3.TowerOfHanoi_V3Character|SetCanMove (Variables|--PrivateAttributes--|GetPRef) true)
  (Variables|/Script/Engine.PlayerController|SetbShowMouseCursor _returnvalue false)
  (Input|SetInputModeGameOnly _returnvalue)
  (Variables|/Game/FirstPersonCPP/Blueprints/FirstPersonCharacter.FirstPersonCharacter_C|SetInGame (Variables|--PrivateAttributes--|GetPRef) false))