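; Timer actor that measures play time while the player character is in game and records it on a win.
; Tick accumulates elapsed time and shows a Timer_UMG widget created through a DoOnce, or zeroes the time and removes the widget when inactive.
; Tick also rebinds the character's WinEvent every frame; the handler disables the timer and saves whole seconds to the game instance's PlayTimeRecord.
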(event Custom|OnWin_Event
  (Variables|--PrivateAttributes--|Setenable false)
  (bind _asmy_thanoi_gminstance (Utilities|Casting|CastToMyTHanoiGMInstance (Game|GetGameInstance)))
  (Variables|/Script/TowerOfHanoi_V3.THanoiGMInstance|SetPlayTimeRecord _asmy_thanoi_gminstance (Math|Float|Truncate (Variables|--PublicAttributes--|GetTime))))

(event EventBeginPlay
  (bind _asfirst_person_character (Utilities|Casting|CastToFirstPersonCharacter (Game|GetPlayerCharacter 0)))
  (Variables|--PrivateAttributes--|SetPRef _asfirst_person_character))

(event Collision|EventActorBeginOverlap
  (params (OtherActor :type Actor%20Object%20Reference)))

(event EventTick
  (params (DeltaSeconds :type Float%20%28single-precision%29))
  (Utilities|FlowControl|Sequence
    (:then_0
      (if (and (Variables|/Game/FirstPersonCPP/Blueprints/FirstPersonCharacter.FirstPersonCharacter_C|GetInGame (Variables|--PrivateAttributes--|GetPRef)) (Variables|--PrivateAttributes--|Getenable))
        (Variables|--PublicAttributes--|SetTime (+ (Variables|--PublicAttributes--|GetTime) (Utilities|Time|GetWorldDeltaSeconds)))
        (Utilities|FlowControl|DoOnce false
          (:Completed
            (bind _returnvalue (UserInterface|CreateWidget "/Game/UMG/Timer_UMG.Timer_UMG_C"))
            (bind _output_get (Variables|--PrivateAttributes--|SetwidgetRef _returnvalue))
            (UserInterface|Viewport|AddtoViewport _output_get 0)))
        (else
          (Variables|--PublicAttributes--|SetTime 0.0)
          (Utilities|IsValid (Variables|--PrivateAttributes--|GetwidgetRef)
            (:Is%20Valid
              (Widget|RemovefromParent (Variables|--PrivateAttributes--|GetwidgetRef))
              (Variables|--PrivateAttributes--|SetwidgetRef 0))))))
    (:then_1
      (EventDispatchers|BindEventtoWinEvent (Variables|--PrivateAttributes--|GetPRef) (delegate Custom|OnWin_Event)))))

(fn ConstructionScript)